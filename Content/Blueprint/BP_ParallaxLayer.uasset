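; BP_ParallaxLayer is a scenery layer actor that shifts along X with the player character to create a side-scrolling parallax effect.
; It records its start location and the player's starting X, then repositions every Tick with Y and Z fixed.
; By default it offsets from its start by player travel scaled by one minus ParallaxRate.
; With FollowCamera set, it instead drifts slightly opposite the player, clamped around world X zero, ignoring its starting X.
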(event `self.ReceiveBeginPlay`
  (set `self.StartLocation` (`self.K2_GetActorLocation`))
  (set `self.PlayerStartX` (.x (`self.K2_GetActorLocation` (`GameplayStatics.GetPlayerCharacter` 0)))))

(event `self.ReceiveTick`
  (params (DeltaSeconds :type "Float (single-precision)"))
  (if (`self.FollowCamera`)
    (`self.K2_SetActorLocation` (`KismetMathLibrary.MakeVector` (- 0.0 (`KismetMathLibrary.FClamp` (* (- (.x (`self.K2_GetActorLocation` (`GameplayStatics.GetPlayerCharacter` 0))) (`self.PlayerStartX`)) 0.03) -40.0 40.0)) (.y (`self.StartLocation`)) (.z (`self.StartLocation`))))
    (else
      (`self.K2_SetActorLocation` (`KismetMathLibrary.MakeVector` (+ (* (- (.x (`self.K2_GetActorLocation` (`GameplayStatics.GetPlayerCharacter` 0))) (`self.PlayerStartX`)) (- 1.0 (`self.ParallaxRate`))) (.x (`self.StartLocation`))) (.y (`self.StartLocation`)) (.z (`self.StartLocation`)))))))

(fn `UserConstructionScript`)