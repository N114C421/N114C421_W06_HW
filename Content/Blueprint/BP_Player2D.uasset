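; BP_Player2D is the player character for a 2D side-view game, driven by Enhanced Input.
; BeginPlay adds the input mapping context and stores the starting position as the respawn location.
; Move input, gated by CanMove, pushes along world X and flips the sprite with negative X scale, while Jump uses the built-in character jump.
; Restart reloads Level01 once GameCompleted is set, and debug prints mark move and jump input.
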(event `EnhancedInput|/Game/Input/IA_Restart`
  (params (ActionValue :type Boolean) (ElapsedSeconds :type "Float (double-precision)") (TriggeredSeconds :type "Float (double-precision)") (InputAction :type "InputAction Object Reference" :default "/Game/Input/IA_Restart.IA_Restart"))
  (:`Started`
    (if (`self.GameCompleted`)
      (`GameplayStatics.OpenLevel` "Level01"))))

(event `EnhancedInput|/Game/Input/IA_Jump`
  (params (ActionValue :type Boolean) (ElapsedSeconds :type "Float (double-precision)") (TriggeredSeconds :type "Float (double-precision)") (InputAction :type "InputAction Object Reference" :default "/Game/Input/IA_Jump.IA_Jump"))
  (:`Started`
    (`self.Jump`)
    (`KismetSystemLibrary.PrintString` "Jump!"))
  (:`Completed`
    (`self.StopJumping`)))

(event `self.ReceiveBeginPlay`
  (`EnhancedInputSubsystemInterface.AddMappingContext` (subsystem `EnhancedInputLocalPlayerSubsystem`) "/Game/Input/IMC_Player.IMC_Player" 0 (struct))
  (set `self.RespawnLocation` (`self.K2_GetActorLocation`)))

(event `EnhancedInput|/Game/Input/IA_Move`
  (params (ActionValue :type "Float (double-precision)") (ElapsedSeconds :type "Float (double-precision)") (TriggeredSeconds :type "Float (double-precision)") (InputAction :type "InputAction Object Reference" :default "/Game/Input/IA_Move.IA_Move"))
  (:`Triggered`
    (if (`self.CanMove`)
      (`self.AddMovementInput` (`KismetMathLibrary.MakeVector` 1.0) ActionValue)
      (if (> ActionValue 0.0)
        (`SceneComponent.SetRelativeScale3D` (`self.Sprite`) (0.05 0.05 0.05))
        (else
          (`SceneComponent.SetRelativeScale3D` (`self.Sprite`) (-0.05 0.05 0.05))))))
  (:`Started`
    (`KismetSystemLibrary.PrintString` "偵測到移動")))

(fn `UserConstructionScript`)